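; Openable door actor that swings open and closed by rotating around its yaw.
; It stores its starting rotation on BeginPlay and responds to OnOpen and OnClose events from an OpenDoor component or interface.
; A timeline lerps yaw from the start to the start minus AngleToOpen, reversing to close.
; An event track on that timeline plays a door lock sound at the door's location.
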(event `self.ReceiveBeginPlay`
  (set `self.InitialRotation` (`self.K2_GetActorRotation`)))

(event `self.OpenDoor.OnOpen`
  (bind (_initialrotation_roll _initialrotation_pitch _initialrotation_yaw) (`KismetMathLibrary.BreakRotator` (`self.InitialRotation`)))
  (bind (_direction _opendoor) (`Timeline|Timeline_0` :!label _label)
    (:`Update`
      (`self.K2_SetActorRotation` (`KismetMathLibrary.MakeRotator` 0.0 0.0 (`KismetMathLibrary.Lerp` _initialrotation_yaw (- _initialrotation_yaw (`self.AngleToOpen`)) _opendoor))))
    (:`NewTrack_1`
      (`GameplayStatics.SpawnSoundAtLocation` "/Game/Audio/door-lock.door-lock" (`self.K2_GetActorLocation`) (struct) 1.0 1.0 0.0 null null))))

(event `self.OpenDoor.OnClose`
  (goto _label :!via `Reverse`))

(fn `UserConstructionScript`)